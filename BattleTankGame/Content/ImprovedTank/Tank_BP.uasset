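; Player-controllable tank Blueprint that handles driving, camera orbit and firing.
; BeginPlay passes the turret and barrel to their reference setters and initialises TankMovement with both tracks.
; Input drives each track's throttle directly or sends forward and turn intent through TankMovement.
; Separate azimuth and attitude gimbals rotate the camera on yaw and pitch, while the fire action calls Fire.
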(event EventBeginPlay
  (Class|Tank|SetTurretReference (Variables|Default|GetTankTurret))
  (Class|Tank|SetBarrelReference (Variables|Default|GetBarrel))
  (Class|TankMovementComponent|Initialise (Variables|Default|GetTankMovement) (Variables|Default|GetLeftTrack) (Variables|Default|GetRightTrack)))

(event Input|ActionEvents|InputActionFire
  (params (Key :type Key%20Structure))
  ;[1 1 1] Aiming&Fire input binding
  (:Pressed
    (Class|Tank|Fire)))

(event Input|AxisEvents|InputAxisCameraAzimuth
  (params (AxisValue :type Float%20%28single-precision%29))
  ;[1 1 1] Aiming&Fire input binding
  (Transformation|AddLocalRotation (Variables|Default|GetAzimuthGimbal) (Math|Rotator|MakeRotator 0.0 0.0 AxisValue) false false))

(event Input|AxisEvents|InputAxisCameraAttitude
  (params (AxisValue :type Float%20%28single-precision%29))
  ;[1 1 1] Aiming&Fire input binding
  (Transformation|AddLocalRotation (Variables|Default|GetAttitudeGimbal) (Math|Rotator|MakeRotator 0.0 AxisValue 0.0) false false))

(event Input|AxisEvents|InputAxisLeftTrackThrottle
  (params (AxisValue :type Float%20%28single-precision%29))
  ;[1 1 1] Tank Moving binding
  (Class|TankTrack|SetThrottle (Variables|Default|GetLeftTrack) AxisValue))

(event Input|AxisEvents|InputAxisRightTrackThrottle
  (params (AxisValue :type Float%20%28single-precision%29))
  ;[1 1 1] Tank Moving binding
  (Class|TankTrack|SetThrottle (Variables|Default|GetRightTrack) AxisValue))

(event Input|AxisEvents|InputAxisForwardAcceleration
  (params (AxisValue :type Float%20%28single-precision%29))
  ;[1 1 1] Tank Moving binding
  (Class|TankMovementComponent|IntendMoveForward (Variables|Default|GetTankMovement) AxisValue))

(event Input|AxisEvents|InputAxisTurnLeft
  (params (AxisValue :type Float%20%28single-precision%29))
  ;[1 1 1] Tank Moving binding
  (Class|TankMovementComponent|IntendMoveLeft (Variables|Default|GetTankMovement) AxisValue))

(fn ConstructionScript)