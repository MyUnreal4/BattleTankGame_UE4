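; Player-drivable tank pawn that hands aiming and movement to TankAiming and TankMovement components, initialised with the barrel, turret and tracks on BeginPlay.
; Input axes rotate the camera gimbals, throttle each track directly or send forward and turn intent to TankMovement; the Fire action calls Fire.
; Component events play a rate-limited throttle sound at world origin and a firing sound outside MainMenu.
; Reload sound logic exists but is disconnected.
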(event EventBeginPlay
  (Class|TankAimingComponent|Initialise (Variables|Default|GetTankAiming) (Variables|Default|GetBarrel) (Variables|Default|GetTankTurret))
  (Class|TankMovementComponent|Initialise (Variables|Default|GetTankMovement) (Variables|Default|GetLTrack) (Variables|Default|GetRTrack)))

(event Accelerate(TankMovement)
  ;[1 1 1] Acceleration Sound
  (Utilities|FlowControl|DoOnce false :!label _label
    (:Completed
      (Audio|PlaySoundatLocation "/Game/ImprovedTank/Throttle_1.Throttle_1" "0, 0, 0" "0, 0, 0" (Math|Float|Clamp(Float) (+ (Math|Float|Absolute(Float) (stale Input|AxisEvents|InputAxisForwardAcceleration AxisValue)) (Math|Float|Absolute(Float) (stale Input|AxisEvents|InputAxisTurnLeft AxisValue)))) 1.0 0.0 0 0 0)
      (Utilities|FlowControl|Delay 0.5)
      (goto _label Reset))))

(event Firing(TankAiming)
  ;[1 1 1] Acceleration Sound
  (bind _returnvalue (Game|GetCurrentLevelName true))
  (if (Utilities|Enum|NotEqual(Enum) _returnvalue "MainMenu")
    (Audio|PlaySoundatLocation "/Game/ImprovedTank/TankFire_1_Cue.TankFire_1_Cue" (Transformation|GetActorLocation self) "0, 0, 0" 1.0 1.0 0.0 0 0 0)))

(event Reloading(TankAiming)
  ;[1 1 1] Acceleration Sound
)

(event Input|ActionEvents|InputActionFire
  (params (Key :type Key%20Structure))
  ;[1 1 1] Aiming&Fire input binding
  (:Pressed
    (Class|Tank|Fire)))

(event Input|AxisEvents|InputAxisCameraAzimuth
  (params (AxisValue :type Float%20%28single-precision%29))
  ;[1 1 1] Aiming&Fire input binding
  (Transformation|AddLocalRotation (Variables|Default|GetAzimuthGimbal) (Math|Rotator|MakeRotator 0.0 0.0 AxisValue) false false))

(event Input|AxisEvents|InputAxisCameraAttitude
  (params (AxisValue :type Float%20%28single-precision%29))
  ;[1 1 1] Aiming&Fire input binding
  (Transformation|AddLocalRotation (Variables|Default|GetAttitudeGimbal) (Math|Rotator|MakeRotator 0.0 AxisValue 0.0) false false))

(event Input|AxisEvents|InputAxisLeftTrackThrottle
  (params (AxisValue :type Float%20%28single-precision%29))
  ;[1 1 1] Tank Moving binding
  (Class|TankTrack|SetThrottle (Variables|Default|GetLTrack) AxisValue))

(event Input|AxisEvents|InputAxisRightTrackThrottle
  (params (AxisValue :type Float%20%28single-precision%29))
  ;[1 1 1] Tank Moving binding
  (Class|TankTrack|SetThrottle (Variables|Default|GetRTrack) AxisValue))

(event Input|AxisEvents|InputAxisForwardAcceleration
  (params (AxisValue :type Float%20%28single-precision%29))
  ;[1 1 1] Tank Moving binding
  (Class|TankMovementComponent|IntendMoveForward (Variables|Default|GetTankMovement) AxisValue))

(event Input|AxisEvents|InputAxisTurnLeft
  (params (AxisValue :type Float%20%28single-precision%29))
  ;[1 1 1] Tank Moving binding
  (Class|TankMovementComponent|IntendMoveLeft (Variables|Default|GetTankMovement) AxisValue))

(fn ConstructionScript)